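; AI pedestrian character that can switch behavior, run to a road and ragdoll on demand.
; On BeginPlay it turns orange, binds to a player delegate that flip-flops the ActivateWandering blackboard key, and polls the plugin's PedestrianDestroyer on timeline updates for distance culling.
; MoveToRoad raises walk speed, moves to a hard-coded Y, plays a montage, then moves on without pathfinding.
; NPCAction events are empty stubs; random material selection is unused.
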(event `Destroy By distance`
  ;[1 1 1] Destroy By Distance From Player
  (`PedestrianDestroyer.DestroyByDistance` (`self.PedestrianDestroyer`) (`self.Distance To Destroy`)) ; Part of the "Pedestrian Destroyer" component from plugin
)

(event `self.ReceiveBeginPlay`
  ;[1 1 1] Bind Delegate from third person character
  (bind _asthird_person_character (cast `/Pedestrian_System/Demo_Content/PlayerCharacter/Blueprints/ThirdPersonCharacter` (`GameplayStatics.GetPlayerCharacter` 0))
    (:`then`
      (add `/Pedestrian_System/Demo_Content/PlayerCharacter/Blueprints/ThirdPersonCharacter.ToggleBehaviorType` _asthird_person_character (delegate `ToggleBehaviorType`)))
    (:`CastFailed`
      _))
  ;[1 1 1] Procedurally Set Material
  (`PrimitiveComponent.SetMaterial` (`self.Mesh`) 0 "/Pedestrian_System/Demo_Content/Materials/CharacterMaterials/MI_CharacterColor_Orange.MI_CharacterColor_Orange")
  ;[1 1 1] Call the Destroy By Distance function on a looped timeline tick *Is Optional in your own project but reccommended for optimization
  (`Timeline|CustomTick`
    (:`Update`
      (`self.Destroy By distance`))))

(event `ToggleBehaviorType`
  (bind _returnvalue (`AIBlueprintHelperLibrary.GetBlackboard` (`AIBlueprintHelperLibrary.GetAIController` self)))
  ;[1 1 1] Toggle blackboard key value for switching behavior types(Delegate from Player) *Can delete only for demo purposes
  (`/Engine/EditorBlueprintResources/StandardMacros.FlipFlop`
    (:`A`
      (`BlackboardComponent.SetValueAsBool` _returnvalue "ActivateWandering" true))
    (:`B`
      (`BlackboardComponent.SetValueAsBool` _returnvalue "ActivateWandering" false))))

(event `NPCActionInterface.NPCAction1`)

(event `NPCActionInterface.NPCAction2`)

(event `MoveToRoad`
  (bind _returnvalue (`AIBlueprintHelperLibrary.GetAIController` self))
  (bind _mesh (`self.Mesh`))
  (bind (_returnvalue_x _returnvalue_y _returnvalue_z) (`KismetMathLibrary.BreakVector` (`SceneComponent.K2_GetComponentLocation` _mesh)))
  (bind (_returnvalue_x_2 _returnvalue_y_2 _returnvalue_z_2) (`KismetMathLibrary.BreakVector` (`SceneComponent.K2_GetComponentLocation` _mesh)))
  (set `CharacterMovementComponent.MaxWalkSpeed` 900.0 (`self.CharacterMovement`))
  (`|AIMoveTo` _returnvalue null (`KismetMathLibrary.MakeVector` _returnvalue_x -35.0 _returnvalue_z) null
    (:`OnSuccess`
      (`|PlayMontage` (`self.Mesh`) (`self.Montage to Play`)
        (:`OnCompleted`
          (`AIController.MoveToLocation` _returnvalue (`KismetMathLibrary.MakeVector` _returnvalue_x_2 -600.0 _returnvalue_z_2) -1.0 true false false true null true))))))

(event `SimulatePhysics`
  (`PrimitiveComponent.SetSimulatePhysics` (`self.Mesh`) true))

(fn `UserConstructionScript`)